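; Wind effect actor that drives the WindMS audio component with a randomly fluctuating wind speed, exposing setters for force, gain and pan.
; Two layers, HSWC and LSWC, each ramp linearly toward a random target around the selected WindForce value, picking a new one when their period expires.
; Box-Muller sampling supplies Gaussian-style periods and targets.
; Each tick sends the summed speed to WindSpeed and prints it.
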(event `self.ReceiveBeginPlay`
  (`self.SetHSWC`)
  (`self.SetLSWC`))

(event `self.ReceiveTick`
  (params (DeltaSeconds :type "Float (single-precision)"))
  (bind _output_get (set `self.FrameTime` DeltaSeconds))
  (bind _output_get_2 (set `self.HSWC_Period` (- (`self.HSWC_Period`) _output_get)))
  (if (< _output_get_2 0.0)
    (`self.SetHSWC`))
  (bind _output_get_3 (set `self.LSWC_Period` (- (`self.LSWC_Period`) (`self.FrameTime`))))
  (if (< _output_get_3 0.0)
    (`self.SetLSWC`))
  (bind _output_get_4 (set `self.HSWC_CurrentSpeed` (`KismetMathLibrary.FMax` (+ (* (`self.HSWC_DeltaSpeed`) (`self.FrameTime`)) (`self.HSWC_CurrentSpeed`)))))
  (bind _output_get_5 (set `self.LSWC_CurrentSpeed` (`KismetMathLibrary.FMax` (+ (* (`self.LSWC_DeltaSpeed`) (`self.FrameTime`)) (`self.LSWC_CurrentSpeed`)) 0.1)))
  (bind _returnvalue (+ _output_get_5 _output_get_4))
  (`KismetSystemLibrary.PrintString` (`KismetStringLibrary.Conv_DoubleToString` _returnvalue))
  (`AudioComponent.SetFloatParameter` (`self.Wind_MS`) "WindSpeed" _returnvalue))

(event `SetWindForce`
  (params (Value :type Integer))
  (set `self.WindForce` Value))

(event `SetGain`
  (params (Value :type "Float (double-precision)"))
  (`AudioComponent.SetFloatParameter` (`self.Wind_MS`) "MasterGain" Value))

(event `SetPan`
  (params (Value :type "Float (double-precision)"))
  (`AudioComponent.SetFloatParameter` (`self.Wind_MS`) "Pan1" Value))

(fn `BoxMuller`
  (returns (Rand1 :type "Float (double-precision)") (Rand2 :type "Float (double-precision)"))
  (bind _returnvalue (* (* (- 1.0 (`KismetMathLibrary.RandomFloat`)) 2.0) (`KismetMathLibrary.GetPI`)))
  (bind _returnvalue_2 (`KismetMathLibrary.Sqrt` (* (`KismetMathLibrary.Loge` (- 1.0 (`KismetMathLibrary.RandomFloat`))) -2.0)))
  (return (* _returnvalue_2 (`KismetMathLibrary.Sin` _returnvalue)) (* _returnvalue_2 (`KismetMathLibrary.Cos` _returnvalue))))

(fn `SetHSWC`
  (bind _output (`|GetArrayItem` (`self.WindForceArray`) (`self.WindForce`)))
  (bind (_rand1 _rand2) (`self.BoxMuller`))
  (bind _output_get (set `self.HSWC_Period` (`KismetMathLibrary.FMax` (+ (* _rand1 (`self.HSWC_SDPeriod`)) (`self.HSWC_MeanPeriod`)) 0.1)))
  (set `self.HSWC_DeltaSpeed` (/ (- (+ (* _rand2 (/ _output 8.0)) _output) (`self.HSWC_CurrentSpeed`)) _output_get)))

(fn `SetLSWC`
  (bind _output (`|GetArrayItem` (`self.WindForceArray`) (`self.WindForce`)))
  (bind (_rand1 _rand2) (`self.BoxMuller`))
  (bind _output_get (set `self.LSWC_Period` (`KismetMathLibrary.FMax` (+ (* _rand1 (`self.LSWC_SDPeriod`)) (`self.LSWC_MeanPeriod`)) 2.0)))
  (set `self.LSWC_DeltaSpeed` (/ (- (+ (* _rand2 (/ _output 8.0)) _output) (`self.LSWC_CurrentSpeed`)) _output_get)))

(fn `UserConstructionScript`)